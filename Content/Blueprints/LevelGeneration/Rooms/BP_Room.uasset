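; Room Blueprint for level generation that gives its walls a random dark color when play begins.
; BeginPlay creates a dynamic instance of M_Solid, randomizes its Base Color within a low RGB range and applies that shared instance to its WallComponents.
; It also prints a debug string; OnConstructionCompleted and the construction script are empty.
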(event `self.ReceiveBeginPlay`
  (`KismetSystemLibrary.PrintString` "CALLED")
  (`|ExecutionSequence`
    (:`then_0`
      (bind _returnvalue (`KismetMaterialLibrary.CreateDynamicMaterialInstance` "/Game/Assets/Materials/M_Solid.M_Solid"))
      (bind _output_get (set `self.WallMaterial` _returnvalue))
      (`MaterialInstanceDynamic.SetVectorParameterValue` _output_get "Base Color" (`KismetMathLibrary.MakeColor` (`KismetMathLibrary.RandomFloatInRange` 0.0 0.25) (`KismetMathLibrary.RandomFloatInRange` 0.0 0.25) (`KismetMathLibrary.RandomFloatInRange` 0.0 0.25)))
      (`PrimitiveComponent.SetMaterial` (`self.K2_GetComponentsByClass` "/Script/ProjectKavun.WallComponent") 0 (`self.WallMaterial`)))))

(event `self.OnConstructionCompleted`)

(fn `UserConstructionScript`)