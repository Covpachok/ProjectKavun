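; BP_EnemyTurret is an enemy turret Blueprint with a Fire function that shoots its Weapon toward the player pawn.
; Fire leads the target by adding a quarter of the player's velocity to their location, then builds the shot rotation from that direction.
; The looping timer that would call Fire is disconnected from any event, and BeginPlay is empty, so nothing in this file triggers firing.
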(event `self.ReceiveBeginPlay`)

(fn `Fire`
  (bind _returnvalue (`GameplayStatics.GetPlayerPawn` 0))
  (bind _returnvalue_2 (`self.K2_GetActorLocation`))
  (bind _returnvalue_3 (- (+ (`self.K2_GetActorLocation` _returnvalue) (/ (`MovementComponent.Velocity` (`self.GetMovementComponent` _returnvalue)) 4.0)) _returnvalue_2))
  (`WeaponComponent.Shoot` (`self.Weapon`) _returnvalue_2 (`KismetMathLibrary.MakeRotFromXY` _returnvalue_3 _returnvalue_3) true))

(fn `UserConstructionScript`)