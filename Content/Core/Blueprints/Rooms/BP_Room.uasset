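; BP_Room is a room actor that handles its wall color, lighting and camera placement for the player.
; On BeginPlay it gives components tagged "Wall" one shared dynamic M_Solid material with a random dark base color.
; When a BP_KavunCharacter enters PlayerDetector, the room snaps that character's CameraActor to its own location and shows its rect lights.
; Leaving the detector hides those lights.
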(event `self.ReceiveBeginPlay`
  (bind _returnvalue (`KismetMaterialLibrary.CreateDynamicMaterialInstance` "/Game/Assets/LevelPrototyping/Materials/M_Solid.M_Solid"))
  (bind _output_get (set `self.WallMaterial` _returnvalue))
  (`MaterialInstanceDynamic.SetVectorParameterValue` _output_get "Base Color" (`KismetMathLibrary.MakeColor` (`KismetMathLibrary.RandomFloatInRange` 0.0 0.25) (`KismetMathLibrary.RandomFloatInRange` 0.0 0.25) (`KismetMathLibrary.RandomFloatInRange` 0.0 0.25)))
  (`PrimitiveComponent.SetMaterial` (`self.GetComponentsByTag` "/Script/Engine.StaticMeshComponent" "Wall") 0 (`self.WallMaterial`)))

(event `self.PlayerDetector.OnComponentBeginOverlap`
  (params (OverlappedComponent :type "PrimitiveComponent Object Reference") (OtherActor :type "Actor Object Reference") (OtherComp :type "PrimitiveComponent Object Reference") (OtherBodyIndex :type Integer) (bFromSweep :type Boolean) (SweepResult :type "HitResult Structure (by ref)"))
  (bind _asbp_kavun_character (cast `/Game/Core/Blueprints/BP_KavunCharacter` OtherActor))
  (`self.K2_SetActorLocation` (`/Game/Core/Blueprints/BP_KavunCharacter.CameraActor` _asbp_kavun_character) (`self.K2_GetActorLocation`) false false)
  (`SceneComponent.SetVisibility` (`self.K2_GetComponentsByClass` "/Script/Engine.RectLightComponent") true false))

(event `self.PlayerDetector.OnComponentEndOverlap`
  (params (OverlappedComponent :type "PrimitiveComponent Object Reference") (OtherActor :type "Actor Object Reference") (OtherComp :type "PrimitiveComponent Object Reference") (OtherBodyIndex :type Integer))
  (cast `/Game/Core/Blueprints/BP_KavunCharacter` OtherActor)
  (`SceneComponent.SetVisibility` (`self.K2_GetComponentsByClass` "/Script/Engine.RectLightComponent") false false))

(fn `UserConstructionScript`)