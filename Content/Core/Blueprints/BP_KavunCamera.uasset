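; BP_KavunCamera is a camera actor that smoothly follows the player's Kavun character.
; On BeginPlay it registers itself as the character's CameraActor and stores that character as FollowTarget, printing an error if the cast fails.
; Every Tick, Follow interpolates the X and Y location at FollowSpeed, with FollowX and FollowY toggling tracking per axis.
; Transition is an empty stub, reached only from unconnected branch logic that never runs.
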(event `self.ReceiveBeginPlay`
  (bind _asbp_kavun_character (cast `/Game/Core/Blueprints/BP_KavunCharacter` (`GameplayStatics.GetPlayerCharacter` 0))
    (:`then`
      (set `/Game/Core/Blueprints/BP_KavunCharacter.CameraActor` self _asbp_kavun_character)
      (set `self.FollowTarget` _asbp_kavun_character))
    (:`CastFailed`
      (`KismetSystemLibrary.PrintString` "Camera: Kavun Character not found!" true true (struct :`R` 1.0 :`B` 0.007763 :`A` 1.0) 10.0))))

(event `self.ReceiveTick`
  (params (DeltaSeconds :type "Float (single-precision)"))
  (`self.Follow` DeltaSeconds))

(fn `Follow`
  (params (DeltaTime :type "Float (double-precision)"))
  (bind (_returnvalue_x _returnvalue_y) (`KismetMathLibrary.BreakVector` (`self.K2_GetActorLocation`)))
  (bind (_returnvalue_x_2 _returnvalue_y_2) (`KismetMathLibrary.BreakVector` (`self.K2_GetActorLocation` (`self.FollowTarget`))))
  (`self.K2_SetActorLocation` (`KismetMathLibrary.MakeVector` (`KismetMathLibrary.FInterpTo` _returnvalue_x (`KismetMathLibrary.SelectFloat` _returnvalue_x_2 _returnvalue_x (`self.bFollowX`)) (`local.DeltaTime`) (`self.FollowSpeed`)) (`KismetMathLibrary.FInterpTo` _returnvalue_y (`KismetMathLibrary.SelectFloat` _returnvalue_y_2 _returnvalue_y (`self.bFollowY`)) (`local.DeltaTime`) (`self.FollowSpeed`)))))

(fn `Transition`)

(fn `UserConstructionScript`)