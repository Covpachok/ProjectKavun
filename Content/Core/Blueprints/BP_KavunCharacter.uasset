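; BP_KavunCharacter is a character Blueprint that creates the stats HUD and controls when its camera actor follows on the X and Y axes.
; On BeginPlay it adds WBP_StatsWidget to the viewport.
; Overlaps on its CameraCollision component call ChangeCameraFollow, which uses CameraColliderX and CameraColliderY component tags to disable following per axis on entry and restore it on exit, printing debug strings.
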(event `self.ReceiveBeginPlay`
  (bind _returnvalue (`|CreateWidget` "/Game/Core/Blueprints/UI/WBP_StatsWidget.WBP_StatsWidget_C"))
  (`UserWidget.AddToViewport` _returnvalue 0))

(event `self.CameraCollision.OnComponentBeginOverlap`
  (params (OverlappedComponent :type "PrimitiveComponent Object Reference") (OtherActor :type "Actor Object Reference") (OtherComp :type "PrimitiveComponent Object Reference") (OtherBodyIndex :type Integer) (bFromSweep :type Boolean) (SweepResult :type "HitResult Structure (by ref)"))
  (`self.ChangeCameraFollow` OtherComp))

(event `self.CameraCollision.OnComponentEndOverlap`
  (params (OverlappedComponent :type "PrimitiveComponent Object Reference") (OtherActor :type "Actor Object Reference") (OtherComp :type "PrimitiveComponent Object Reference") (OtherBodyIndex :type Integer))
  (`self.ChangeCameraFollow` OtherComp true))

(fn `ChangeCameraFollow`
  (params (Collision :type "ActorComponent Object Reference") (bShouldFollow :type Boolean))
  (`|ExecutionSequence`
    (:`then_0`
      (if (`ActorComponent.ComponentHasTag` Collision "CameraColliderX")
        (set `/Game/Core/Blueprints/BP_KavunCamera.bFollowX` (`local.bShouldFollow`) (`self.CameraActor`))
        (`KismetSystemLibrary.PrintString` "FollowX")))
    (:`then_1`
      (if (`ActorComponent.ComponentHasTag` Collision "CameraColliderY")
        (set `/Game/Core/Blueprints/BP_KavunCamera.bFollowY` (`local.bShouldFollow`) (`self.CameraActor`))
        (`KismetSystemLibrary.PrintString` "FollowY")))))

(fn `UserConstructionScript`)