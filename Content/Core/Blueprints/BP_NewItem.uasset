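; BP_NewItem is an item that trades damage for fire rate on a KavunCharacter.
; Its Sphere overlap casts the actor and jumps into the logic shared with OnAddedtoInventory, setting projectiles-per-second and damage multipliers and reducing Damage through the attributes component.
; The inventory add and hide branch is disconnected, so the item stays in place and each overlap lowers Damage again.
; Only the overlap path sets the character reference that OnAddedtoInventory uses.
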(event `self.OnAddedToInventory`
  (params (InventoryOwner :type "KavunCharacter Object Reference"))
  (bind _returnvalue (`KavunCharacter.GetAttributesComponent` (stale `self.Sphere.OnComponentBeginOverlap` _askavun_character)))
  (`/Engine/EditorBlueprintResources/StandardMacros.IsValid` _returnvalue :!label _label
    (:`Is Valid`
      (`CharacterAttributesComponent.SetAttributeBase` _returnvalue "ECharacterAttributes_ProjectilesPerSecondMultiplier" 4.0)
      (`CharacterAttributesComponent.ChangeAttribute` _returnvalue "ECharacterAttributes_Damage" -1.0)
      (`CharacterAttributesComponent.SetAttributeBase` _returnvalue "ECharacterAttributes_DamageMultiplier" 0.25))))

(event `self.Sphere.OnComponentBeginOverlap`
  (params (OverlappedComponent :type "PrimitiveComponent Object Reference") (OtherActor :type "Actor Object Reference") (OtherComp :type "PrimitiveComponent Object Reference") (OtherBodyIndex :type Integer) (bFromSweep :type Boolean) (SweepResult :type "HitResult Structure (by ref)"))
  (bind _askavun_character (cast `KavunCharacter` OtherActor))
  (goto _label))

(fn `UserConstructionScript`)