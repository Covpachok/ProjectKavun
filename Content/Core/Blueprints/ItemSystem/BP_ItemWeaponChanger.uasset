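; Item Blueprint that modifies the player's weapon stats while it is held.
; On pickup it finds the player's WeaponComponent and passes its ShotDelay and ProjectileSpeed values to ChangeShotDelay and ChangeProjectileSpeed.
; On drop it passes the negated values to the same functions, so the modifiers act as reversible deltas.
; Both events do nothing if the player has no valid WeaponComponent.
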(event `self.ReceiveBeginPlay`
  (`parent.ReceiveBeginPlay`))

(event `self.OnPickedUp_Event`
  (params (Player :type "/Game/Core/Blueprints/BP_KavunCharacter Object Reference"))
  (bind _returnvalue (`self.GetComponentByClass` Player "/Script/ProjectKavun.WeaponComponent"))
  (`/Engine/EditorBlueprintResources/StandardMacros.IsValid` _returnvalue
    (:`Is Valid`
      (`WeaponComponent.ChangeShotDelay` _returnvalue (`self.ShotDelay`))
      (`WeaponComponent.ChangeProjectileSpeed` _returnvalue (`self.ProjectileSpeed`)))))

(event `self.OnDropped_Event`
  (params (Player :type "/Game/Core/Blueprints/BP_KavunCharacter Object Reference"))
  (bind _returnvalue (`self.GetComponentByClass` Player "/Script/ProjectKavun.WeaponComponent"))
  (`/Engine/EditorBlueprintResources/StandardMacros.IsValid` _returnvalue
    (:`Is Valid`
      (`WeaponComponent.ChangeShotDelay` _returnvalue (* (`self.ShotDelay`) -1.0))
      (`WeaponComponent.ChangeProjectileSpeed` _returnvalue (* (`self.ProjectileSpeed`) -1.0)))))

(fn `UserConstructionScript`
  (`parent.UserConstructionScript`))