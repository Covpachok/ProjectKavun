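; BP_Inventory is an inventory component that lets its owning actor pick up and drop world items.
; It stores item info in a map keyed by item Id, so AddItem ignores an Id already held, and otherwise notifies the item and destroys its actor.
; RemoveItem respawns the stored class at the owner's transform, fires the dropped event and removes the entry.
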(fn `AddItem`
  (params (Item :type "/Game/Core/Blueprints/ItemSystem/BP_Item Object Reference"))
  (bind (_iteminfo_name _iteminfo_id) (break `/Game/Core/Blueprints/ItemSystem/S_ItemInfo` (`/Game/Core/Blueprints/ItemSystem/BP_Item.ItemInfo` Item)))
  (if (not (`BlueprintMapLibrary.Map_Contains` (`self.Items`) _iteminfo_id))
    (`BlueprintMapLibrary.Map_Add` (`self.Items`) _iteminfo_id (`/Game/Core/Blueprints/ItemSystem/BP_Item.ItemInfo` (`local.Item`)))
    (`/Game/Core/Blueprints/ItemSystem/BP_Item.OnPickedUp_Event` (`local.Item`) (`self.Owner`))
    (`Actor.K2_DestroyActor` (`local.Item`))))

(fn `RemoveItem`
  (params (Id :type Integer))
  (locals (ItemId :type Integer))
  (bind (_value _returnvalue) (`BlueprintMapLibrary.Map_Find` (`self.Items`) Id))
  (set `local.ItemId` Id)
  (if _returnvalue
    (bind _returnvalue_2 (`|SpawnActorFromClass` (`.Class_8_5F9F485C44692C6A8422049554CD6CD6` (break `/Game/Core/Blueprints/ItemSystem/S_ItemInfo` _value)) (`Actor.GetTransform` (`self.GetOwner`)) "Undefined" "MultiplyWithRoot" null null))
    (`/Game/Core/Blueprints/ItemSystem/BP_Item.OnDropped_Event` _returnvalue_2 (`self.Owner`))
    (`BlueprintMapLibrary.Map_Remove` (`self.Items`) (`local.ItemId`))))