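; Main game mode that forces a low-cost graphics profile whenever play begins.
; BeginPlay sets the game user settings to windowed mode at full resolution scale with dynamic resolution enabled, then applies the resolution.
; It then drops the main scalability groups, such as shadows, textures, global illumination and effects, to their lowest level and applies the settings, overriding previous choices.
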(event `self.ReceiveBeginPlay`
  (bind _returnvalue (`GameUserSettings.GetGameUserSettings`))
  (`GameUserSettings.SetFullscreenMode` _returnvalue "Windowed")
  (`GameUserSettings.SetResolutionScaleNormalized` _returnvalue 1.0)
  (`GameUserSettings.SetDynamicResolutionEnabled` _returnvalue true)
  (`GameUserSettings.ApplyResolutionSettings` _returnvalue true)
  (`GameUserSettings.SetPostProcessingQuality` _returnvalue 0)
  (`GameUserSettings.SetShadowQuality` _returnvalue 0)
  (`GameUserSettings.SetTextureQuality` _returnvalue 0)
  (`GameUserSettings.SetGlobalIlluminationQuality` _returnvalue 0)
  (`GameUserSettings.SetReflectionQuality` _returnvalue 0)
  (`GameUserSettings.SetVisualEffectQuality` _returnvalue 0)
  (`GameUserSettings.SetAntiAliasingQuality` _returnvalue 0)
  (`GameUserSettings.SetViewDistanceQuality` _returnvalue 0)
  (`GameUserSettings.ApplySettings` _returnvalue true))

(fn `UserConstructionScript`)