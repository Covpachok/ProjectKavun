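; Level-generation room actor that tints its walls a random dark color and spawns a random decoration once construction completes.
; Decoration rows from DT_RoomDecorations are picked at random and retried, with a capped attempt count, until one matches the room's Shape.
; Player detector overlaps are counted so overlapping detectors trigger enter and exit only once.
; Entering calls the camera's ChangeFollow, moves it to the room and shows rect lights, which exiting hides.
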(event `self.ReceiveBeginPlay`)

(event `self.OnConstructionCompleted`
  (bind _shape (`self.Shape`))
  (`|ExecutionSequence`
    (:`then_0`
      (bind _returnvalue (`KismetMaterialLibrary.CreateDynamicMaterialInstance` "/Game/Assets/LevelPrototyping/Materials/M_Solid.M_Solid" "іфNone"))
      (bind _output_get (set `self.WallMaterial` _returnvalue))
      (`MaterialInstanceDynamic.SetVectorParameterValue` _output_get "Base Color" (`KismetMathLibrary.MakeColor` (`KismetMathLibrary.RandomFloatInRange` 0.0 0.25) (`KismetMathLibrary.RandomFloatInRange` 0.0 0.25) (`KismetMathLibrary.RandomFloatInRange` 0.0 0.25)))
      (`PrimitiveComponent.SetMaterial` (`self.GetComponentsByTag` "/Script/Engine.StaticMeshComponent" "Wall") 0 (`self.WallMaterial`)))
    (:`then_1`
      (bind _outrownames (`DataTableFunctionLibrary.GetDataTableRowNames` "/Game/Core/Blueprints/LevelGeneration/Rooms/DT_RoomDecorations.DT_RoomDecorations" :!label _label))
      (bind _returnvalue_2 (`|GetDataTableRow` "/Game/Core/Blueprints/LevelGeneration/Rooms/DT_RoomDecorations.DT_RoomDecorations" (`|GetArrayItem` _outrownames (`KismetMathLibrary.RandomIntegerInRange` 0 (- (`KismetArrayLibrary.Array_Length` _outrownames) 1))))
        (:`then`
          (`KismetSystemLibrary.PrintString` (`|GetEnumeratorNameAsString` _shape))
          (bind (_roomtype _roomshape _class) (break `/Game/Core/Blueprints/LevelGeneration/Rooms/S_RoomDecorationInfo` _returnvalue_2))
          (if (`|EnumEquality` _roomshape _shape)
            (`|SpawnActorFromClass` _class (`KismetMathLibrary.MakeTransform` (`self.K2_GetActorLocation`)) "Undefined" "MultiplyWithRoot" null null)
            (else
              (`KismetSystemLibrary.PrintString` "FUCK")
              (bind _result (`/Engine/EditorBlueprintResources/StandardMacros.IncrementInt` (`self.OverflowCounter`))
                (:`  `
                  (if (> _result 10)
                    (`KismetSystemLibrary.PrintString` "I'm done")
                    (else
                      (goto _label))))))))
        (:`RowNotFound`
          (`KismetSystemLibrary.PrintString` "For some reason didn't found any decorations"))))))

(event `self.PlayerDetector.OnComponentBeginOverlap`
  (params (OverlappedComponent :type "PrimitiveComponent Object Reference") (OtherActor :type "Actor Object Reference") (OtherComp :type "PrimitiveComponent Object Reference") (OtherBodyIndex :type Integer) (bFromSweep :type Boolean) (SweepResult :type "HitResult Structure (by ref)"))
  (`self.OnDetectorOverlapBegin` OtherActor))

(event `self.PlayerDetector.OnComponentEndOverlap`
  (params (OverlappedComponent :type "PrimitiveComponent Object Reference") (OtherActor :type "Actor Object Reference") (OtherComp :type "PrimitiveComponent Object Reference") (OtherBodyIndex :type Integer))
  (`self.OnDetectorOverlapEnd` OtherActor))

(event `PlayerEnteredRoom`
  (params (Player :type "/Game/Core/Blueprints/BP_KavunCharacter Object Reference"))
  (bind _returnvalue (`KavunCharacter.GetCameraActor` Player))
  (`KavunCamera.ChangeFollow` _returnvalue true)
  (`self.K2_SetActorLocation` _returnvalue (`self.K2_GetActorLocation`) false true)
  (`SceneComponent.SetVisibility` (`self.K2_GetComponentsByClass` "/Script/Engine.RectLightComponent") true false))

(event `PlayerExitedRoom`
  (params (Player :type "/Game/Core/Blueprints/BP_KavunCharacter Object Reference"))
  (`SceneComponent.SetVisibility` (`self.K2_GetComponentsByClass` "/Script/Engine.RectLightComponent") false false))

(fn `OnDetectorOverlapBegin`
  (params (OverlappedActor :type "Actor Object Reference"))
  (bind _asbp_kavun_character (cast `/Game/Core/Blueprints/BP_KavunCharacter` OverlappedActor))
  ;[0.2199 0.2734 1] In case player was detected by other detectors
  (bind _result (`/Engine/EditorBlueprintResources/StandardMacros.IncrementInt` (`self.PlayerDetectedCount`))
    (:`  `
      (if (== _result 1)
        (`self.PlayerEnteredRoom` _asbp_kavun_character)))))

(fn `OnDetectorOverlapEnd`
  (params (OverlappedActor :type "Actor Object Reference"))
  (bind _asbp_kavun_character (cast `/Game/Core/Blueprints/BP_KavunCharacter` OverlappedActor))
  ;[0.8157 0.3707 1] In case player was detected by other detectors
  (bind _result (`/Engine/EditorBlueprintResources/StandardMacros.DecrementInt` (`self.PlayerDetectedCount`))
    (:`  `
      (if (== _result 0)
        (`self.PlayerExitedRoom` _asbp_kavun_character)))))

(fn `UserConstructionScript`)